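; BP_TV is an animated TV creature that starts walking the first time an interactor hovers it, which is allowed from a distance.
; InterpToMovement drives the walk, with a timeline rotating the mesh on reversals and projection animations playing when movement stops.
; OnHit drains health until a death animation and delayed destroy.
; Tick shows the TextRender only while the gameplay parameter collection's brightness is below a threshold.
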(event `self.ReceiveBeginPlay`
  (bind _interptomovement (`self.InterpToMovement`))
  (set `self.StartLocation` (`self.K2_GetActorLocation`))
  (`MovementComponent.StopMovementImmediately` _interptomovement)
  (add `InterpToMovementComponent.OnInterpToReverse` _interptomovement (delegate `OnReverse`))
  (`TimelineComponent.SetPlayRate` (`self.TimelineRotation`) (`self.RotationSpeed`))
  (add `InterpToMovementComponent.OnInterpToStop` _interptomovement (delegate `OnStopWalking`)))

(event `OnReverse`
  (params (ImpactResult :type "HitResult Structure (by ref)") (Time :type "Float (single-precision)"))
  (if (not (`self.bDead`))
    (set `self.bFlipForward` (not (`self.bFlipForward`)))
    (`self.OnRotate`)))

(event `OnStopWalking`
  (params (ImpactResult :type "HitResult Structure (by ref)") (Time :type "Float (single-precision)"))
  (`SkeletalMeshComponent.PlayAnimation` (`self.SkeletalMesh`) "/Game/BehaviorGJ/Anim/TV/Anim_TV_ProjectionStart.Anim_TV_ProjectionStart" false)
  (`KismetSystemLibrary.Delay` 1.0)
  (`SkeletalMeshComponent.PlayAnimation` (`self.SkeletalMesh`) "/Game/BehaviorGJ/Anim/TV/Anim_TV_ProjectionLoop.Anim_TV_ProjectionLoop" true))

(event `self.ReceiveTick`
  (params (DeltaSeconds :type "Float (single-precision)"))
  (if (not (`self.bDead`))
    (bind _returnvalue (`KismetMaterialLibrary.GetScalarParameterValue` "/Game/Core/MPC_Gameplay.MPC_Gameplay" "Brigthness"))
    (`SceneComponent.SetVisibility` (`self.TextRender`) (< _returnvalue 0.9) false)))

(event `OnRotate`
  (bind _returnvalue (`self.K2_GetActorRotation`))
  (if (`self.bDead`)
    _
    (elif (`self.bFlipForward`)
      (bind (_direction _alpha) (`Timeline|TimelineRotation` :!via `PlayFromStart` :!label _label)
        (:`Update`
          (`SceneComponent.K2_SetWorldRotation` (`self.SkeletalMesh`) (`KismetMathLibrary.RLerp` _returnvalue (`KismetMathLibrary.MakeRotator` (.roll _returnvalue) (.pitch _returnvalue) 180.0) _alpha (`self.bFlipForward`)) false false)))
      (else
        (goto _label :!via `ReverseFromEnd`)))))

(event `OnStartMoving`
  (bind (_returnvalue_x _returnvalue_y) (`KismetMathLibrary.BreakVector` (`self.K2_GetActorLocation`)))
  (bind (_startlocation_x _startlocation_y _startlocation_z) (`KismetMathLibrary.BreakVector` (`self.StartLocation`)))
  (bind (_returnvalue_x_2 _returnvalue_y_2) (`KismetMathLibrary.BreakVector` (+ (`self.StartLocation`) (0.0 500.0 0.0))))
  (if (not (`self.bDead`))
    (bind (_direction _alpha) (`Timeline|MoveTowardsPoint` :!via `PlayFromStart`)
      (:`Update`
        (`self.K2_SetActorLocation` (`KismetMathLibrary.VLerp` (`KismetMathLibrary.MakeVector` _returnvalue_x _returnvalue_y _startlocation_z) (`KismetMathLibrary.MakeVector` _returnvalue_x_2 _returnvalue_y_2 _startlocation_z) (* (* _alpha (`GameplayStatics.GetWorldDeltaSeconds`)) (`self.RotationSpeed`))))))))

(event `/Game/Core/BPI_Interacatable.OnHit`
  (params (Actor :type "Actor Object Reference") (Hit :type "HitResult Structure"))
  (if (not (`self.bDead`))
    (bind _result (`/Engine/EditorBlueprintResources/StandardMacros.DecrementInt` (`self.HealthPoints`))
      (:`  `
        (if (<= _result 0)
          (`SkeletalMeshComponent.PlayAnimation` (`self.SkeletalMesh`) "/Game/BehaviorGJ/Anim/TV/Anim_TV_Death2.Anim_TV_Death2" false)
          (set `self.bDead` true)
          (`KismetSystemLibrary.Delay` 2.5)
          (`self.K2_DestroyActor`))))))

(fn `CanInteractFromDistance`
  (params (Interactor :type "Actor Object Reference"))
  (returns (bCanInteract :type Boolean))
  (return true))

(fn `OnInteractHover`
  (params (Interactor :type "Actor Object Reference"))
  (returns (bShouldFocus :type Boolean))
  (if (not (`self.bAnimated`))
    (set `self.bAnimated` true)
    (`InterpToMovementComponent.RestartMovement` (`self.InterpToMovement`) 1.0)
    (`SkeletalMeshComponent.PlayAnimation` (`self.SkeletalMesh`) "/Game/BehaviorGJ/Anim/TV/Anim_TV_Marche.Anim_TV_Marche" true)
    (return true)))

(fn `UserConstructionScript`)