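; BP_Door is an interactable door that shows a widget on hover and opens when used.
; Hovering shows the widget if the interactor is within InteractionDistance and the door is not yet Activated.
; Interacting plays the open animation on the skeletal mesh, disables collider collision, sets Activated and hides the widget.
; Exiting interaction also hides the widget, and the file contains no closing logic.
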(event `self.ReceiveBeginPlay`
  (`SceneComponent.SetVisibility` (`self.Widget`) false false))

(event `OnShowWidget`
  (`SceneComponent.SetVisibility` (`self.Widget`) true false))

(event `OnOpen`
  (`SkeletalMeshComponent.PlayAnimation` (`self.SkeletalMesh`) "/Game/BehaviorGJ/Anim/Anim_Door_Open.Anim_Door_Open" false)
  (`PrimitiveComponent.SetCollisionEnabled` (`self.Collider`) "NoCollision")
  (set `self.bActivated` true))

(event `/Game/Core/BPI_Interacatable.OnInteractDo`
  (`self.OnOpen`)
  (`SceneComponent.SetVisibility` (`self.Widget`) false false :!label _label))

(event `/Game/Core/BPI_Interacatable.OnInteractExit`
  (goto _label))

(fn `CanInteractFromDistance`
  (params (Interactor :type "Actor Object Reference"))
  (returns (bCanInteract :type Boolean))
  (return (<= (`KismetMathLibrary.Vector_Distance` (`self.K2_GetActorLocation` Interactor) (`self.K2_GetActorLocation`)) (`self.InteractionDistance`))))

(fn `OnInteractHover`
  (params (Interactor :type "Actor Object Reference"))
  (returns (bShouldFocus :type Boolean))
  (if (<= (`KismetMathLibrary.Vector_Distance` (`self.K2_GetActorLocation`) (`self.K2_GetActorLocation` Interactor)) (`self.InteractionDistance`))
    (if (not (`self.bActivated`))
      (`self.OnShowWidget`)
      (return false))))

(fn `UserConstructionScript`)