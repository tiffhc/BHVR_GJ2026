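; Player controller that handles first-level input and the pause/settings menu for BP_MainCharacter.
; On possess it adds the Enhanced Input mapping and caches the character; look and move drive the pawn unless PauseMenu is set.
; The pause action toggles that flag, the WBP_Settings widget and mouse cursor, without pausing the game.
; The widget's brightness event updates the character and scales spotlights on "Brightness"-tagged actors, with a minimum intensity.
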(event `self.ReceiveBeginPlay`)

(event `self.ReceivePossess`
  (params (PossessedPawn :type "Pawn Object Reference"))
  (`EnhancedInputSubsystemInterface.AddMappingContext` (subsystem `EnhancedInputLocalPlayerSubsystem`) "/Game/Core/Inputs/IMC_Main.IMC_Main" 0 (struct))
  (bind _asbp_main_character (cast `/Game/Core/BP_MainCharacter` PossessedPawn))
  (set `self.Player_Ref` _asbp_main_character))

(event `EnhancedInput|/Game/Core/Inputs/IA_Look`
  (params (ActionValue :type "Vector2D Structure") (ElapsedSeconds :type "Float (double-precision)") (TriggeredSeconds :type "Float (double-precision)") (InputAction :type "InputAction Object Reference" :default "/Game/Core/Inputs/IA_Look.IA_Look"))
  (:`Triggered`
    (if (not (`self.bPauseMenu`))
      (`Pawn.AddControllerYawInput` (`GameplayStatics.GetPlayerPawn` 0) ActionValue_X)
      (`Pawn.AddControllerPitchInput` (`GameplayStatics.GetPlayerPawn` 0) ActionValue_Y))))

(event `EnhancedInput|/Game/Core/Inputs/IA_Move`
  (params (ActionValue :type "Vector2D Structure") (ElapsedSeconds :type "Float (double-precision)") (TriggeredSeconds :type "Float (double-precision)") (InputAction :type "InputAction Object Reference" :default "/Game/Core/Inputs/IA_Move.IA_Move"))
  (bind _returnvalue (`GameplayStatics.GetPlayerPawn` 0))
  (bind _returnvalue_2 (`GameplayStatics.GetPlayerPawn` 0))
  (:`Triggered`
    (if (not (`self.bPauseMenu`))
      (`Pawn.AddMovementInput` _returnvalue_2 (`self.GetActorRightVector` _returnvalue_2) ActionValue_X false)
      (`Pawn.AddMovementInput` _returnvalue (`self.GetActorForwardVector` _returnvalue) ActionValue_Y false))))

(event `EnhancedInput|/Game/Core/Inputs/IA_Pause`
  (params (ActionValue :type Boolean) (ElapsedSeconds :type "Float (double-precision)") (TriggeredSeconds :type "Float (double-precision)") (InputAction :type "InputAction Object Reference" :default "/Game/Core/Inputs/IA_Pause.IA_Pause"))
  (:`Started`
    (bind _output_get (set `self.bPauseMenu` (not (`self.bPauseMenu`))))
    (if _output_get
      (bind _returnvalue (`|CreateWidget` "/Game/BehaviorGJ/UI/WBP_Settings.WBP_Settings_C"))
      (bind _output_get_2 (set `self.WBP_Settings` _returnvalue))
      (`UserWidget.AddToViewport` _output_get_2 0)
      (set `self.bShowMouseCursor` true)
      (add `/Game/BehaviorGJ/UI/WBP_Settings.OnBrigthnessUpdated` (`self.WBP_Settings`) (delegate `OnUpdateBrightness`))
      (else
        (bind _wbp_settings (`self.WBP_Settings`)
          (:`then`
            (`Widget.RemoveFromParent` _wbp_settings)
            (set `self.bShowMouseCursor` false))
          (:`else`))))))

(event `OnUpdateBrightness`
  (params (Value :type "Float (double-precision)"))
  (`/Game/Core/BP_MainCharacter.SetBrightness` (`self.Player_Ref`) Value)
  (bind _outactors (`GameplayStatics.GetAllActorsWithTag` "Brightness"))
  (for _array_element _outactors
    (`LightComponent.SetIntensity` (`self.GetComponentByClass` _array_element "/Script/Engine.SpotLightComponent") (`KismetMathLibrary.FMax` (* 120.0 Value) 85.0))))

(fn `UserConstructionScript`)