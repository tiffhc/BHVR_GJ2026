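; Main player character that focuses and uses nearby interactables, swings an axe and forwards settings requests to its controller.
; Each tick a sphere trace ahead finds interactables, sends hover and exit messages, and drives controller focus.
; A timeline rolls the weapon while a delayed sphere trace at StrikePoint sends hit messages, with a flag blocking overlapping swings.
; Brightness is set by clamping the camera's post-process exposure range.
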(event `self.ReceiveBeginPlay`
  (`self.SetBrightness` 1.0)
  (set `self.DefaultWeaponRotation` (`SceneComponent.RelativeRotation` (`self.Weapon`)))
  (set `self.DefaultWeaponLocation` (`SceneComponent.RelativeLocation` (`self.Weapon`)))
  (`TimelineComponent.SetPlayRate` (`self.TimelineSwingAxe`) 1.8))

(event `SetBrightness`
  (params (Value :type "Float (double-precision)"))
  (bind _returnvalue (`KismetMathLibrary.FClamp` (- 10.0 (* Value 10.0)) 0.0 7.0))
  (setmembers `PostProcessSettings` :`StructRef` (`CameraComponent.PostProcessSettings` (`self.Camera`)) :`AutoExposureMinBrightness` (- _returnvalue 0.1) :`AutoExposureMaxBrightness` (+ _returnvalue 0.1)))

(event `self.ReceiveTick`
  (params (DeltaSeconds :type "Float (single-precision)"))
  (`self.ComputeInteractions`))

(event `OnTryInteraction`
  (bind _currentinteractable (`self.CurrentInteractable`)
    (:`then`
      (message `/Game/Core/BPI_Interacatable.OnInteractDo` _currentinteractable))
    (:`else`)))

(event `/Game/Core/BPI_Player.OnOpenSettings`
  (`/Game/Core/BP_PlayerController.OnOpenSettings` (`self.PlayerController_Ref`)))

(event `OnSwingAxe`
  (if (not (`self.bSwung`))
    (set `self.bSwung` true)
    (`TimelineComponent.PlayFromStart` (`self.TimelineSwingAxe`))
    (`KismetSystemLibrary.Delay` 0.2)
    (`self.ComputeAttack`)))

(fn `ComputeAttack`
  (bind _returnvalue (`SceneComponent.K2_GetComponentLocation` (`self.StrikePoint`)))
  (bind (_outhit _returnvalue_2) (`KismetSystemLibrary.SphereTraceSingleForObjects` _returnvalue _returnvalue 26.0 (`|MakeArray` "ObjectTypeQuery2" :!type "EObjectTypeQuery Enum")))
  (if _returnvalue_2
    (message `/Game/Core/BPI_Interacatable.OnHit` (`.HitActor` (`GameplayStatics.BreakHitResult` _outhit)) self _outhit)))

(fn `ComputeInteractions`
  (bind _returnvalue (+ (`self.K2_GetActorLocation`) (* (`self.GetActorForwardVector`) 100.0)))
  (bind (_outhits _returnvalue_2) (`KismetSystemLibrary.SphereTraceMultiForObjects` _returnvalue _returnvalue 625.0 (`|MakeArray` "ObjectTypeQuery2" :!type "EObjectTypeQuery Enum")))
  (if _returnvalue_2
    (for _array_element _outhits
      (bind (_bblockinghit _binitialoverlap _time _distance _location _impactpoint _normal _impactnormal _physmat _hitactor) (`GameplayStatics.BreakHitResult` _array_element))
      (bind _bcaninteract (message `/Game/Core/BPI_Interacatable.CanInteractFromDistance` _hitactor self))
      (if _bcaninteract
        (bind _currentinteractable (`self.CurrentInteractable`)
          (:`then`
            (if (!= _currentinteractable (`self.CurrentInteractable`))
              (message `/Game/Core/BPI_Interacatable.OnInteractExit` _currentinteractable)))
          (:`else`
            _))
        (bind _output_get (set `self.CurrentInteractable` _hitactor))
        (bind _bshouldfocus (message `/Game/Core/BPI_Interacatable.OnInteractHover` _output_get self))
        (if _bshouldfocus
          (`/Game/Core/BP_PlayerController.OnStartFocus` (`self.PlayerController_Ref`)))
        (else
          (bind _currentinteractable_2 (`self.CurrentInteractable` :!label _label)
            (:`then`
              (if (== _hitactor _currentinteractable_2)
                (message `/Game/Core/BPI_Interacatable.OnInteractExit` _currentinteractable_2)
                (set `self.CurrentInteractable` null)))
            (:`else`)))))
    (else
      (`/Game/Core/BP_PlayerController.OnEndFocus` (`self.PlayerController_Ref`))
      (goto _label))))

(fn `IsFocusing`
  (returns (bFocus :type Boolean))
  (return (`/Game/Core/BP_PlayerController.bFocus` (`self.PlayerController_Ref`))))

(fn `UserConstructionScript`)